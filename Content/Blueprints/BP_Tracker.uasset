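; BP_Tracker is a race tracker Blueprint that hands lap settings to the player controller and starts game setup.
; On BeginPlay it caches BP_PlayerController, copies MaxLaps to it, calls UpdateTimes and StartGameSetup, then runs StartSequence.
; The checkpoint loop in StartSequence is empty, and the timing, lap and checkpoint functions are stubs, with RaceCompleteCheck always returning false.
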(event Custom|ApplySettings
  (bind _playercontroller (Variables|Default|GetPlayerController))
  ;[1 1 1] Apply User Settings in Starting a Game
  (Variables|/Game/Blueprints/BP_PlayerController.BP_PlayerController_C|SetMaxLaps _playercontroller (Variables|CustomSettings|GetMaxLaps))
  (CallFunction|UpdateTimes)
  (Default|StartGameSetup _playercontroller))

(event Custom|StartSequence
  (for _array_element (Variables|Checkpoints|GetCheckpoints)
    _))

(event EventBeginPlay
  (bind _asbp_player_controller (Utilities|Casting|CastToBP_PlayerController (Game|GetPlayerController 0)))
  (Variables|Default|SetPlayerController _asbp_player_controller)
  (CallFunction|ApplySettings)
  (CallFunction|StartSequence))

(fn ConstructionScript)

(fn UpdateTimes)

(fn LapCheck
  (params (Checkpoint :type Integer)))

(fn ActivateCheckpoint
  (params (NextCheckpoint :type BP%20Checkpoint%20Object%20Reference)))

(fn RaceCompleteCheck
  (return false))